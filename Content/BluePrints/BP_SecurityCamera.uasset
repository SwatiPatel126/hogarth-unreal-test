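; BP_SecurityCamera is a security camera that shows player detection through its spotlight color.
; Every tick it checks the player's distance to CenterPoint against DetectionRadius, then uses a dot product and arccosine to get the viewing angle.
; The light turns red within FrontalAngle, yellow within SideAngle and green otherwise.
; The angle is subtracted from 180, so both cones center on CenterPoint's negative forward vector.
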(event `self.ReceiveTick`
  (params (DeltaSeconds :type "Float (single-precision)"))
  (bind _centerpoint (`self.centerPoint`))
  (bind _spotlight (`self.SpotLight`))
  (bind _returnvalue (`self.K2_GetActorLocation` (`GameplayStatics.GetPlayerCharacter` 0)))
  (bind _returnvalue_2 (`SceneComponent.K2_GetComponentLocation` _centerpoint))
  (if (<= (`KismetMathLibrary.Vector_Distance` _returnvalue _returnvalue_2) (`self.DetectionRadius`))
    (bind _direction (`self.GetDirection` _returnvalue_2 _returnvalue))
    (bind _returnvalue_3 (- 180.0 (`KismetMathLibrary.RadiansToDegrees` (`KismetMathLibrary.Acos` (`KismetMathLibrary.Dot_VectorVector` (`SceneComponent.GetForwardVector` _centerpoint) _direction)))))
    (if (<= _returnvalue_3 (`self.FrontalAngle`))
      (`LightComponent.SetLightColor` _spotlight (struct :`R` 1.0 :`A` 1.0) true)
      (elif (<= _returnvalue_3 (`self.SideAngle`))
        (`LightComponent.SetLightColor` _spotlight (struct :`R` 1.0 :`G` 1.0 :`A` 1.0) true)
        (else
          (`LightComponent.SetLightColor` _spotlight (struct :`G` 1.0 :`A` 1.0) true :!label _label))))
    (else
      (goto _label))))

(fn `GetDirection`
  (params (from :type "Vector Structure") (to :type "Vector Structure"))
  (returns (Direction :type "Vector Structure"))
  (return (`KismetMathLibrary.Normal` (- to from))))

(fn `UserConstructionScript`)